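; Wandering pedestrian character that idles, chats with other pedestrians and leaps away from the player.
; A self-repeating MoveAround loop issues random-direction AI moves only while recently rendered, despite the check's PlayerDistance name.
; Failed moves trigger an idle montage branch and a chance to talk when Dialogue_box has flagged a pedestrian, though those montages are unset.
; Playeravoidance overlap launches the character once per contact; the scream logic is disconnected.
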(event `self.ReceiveBeginPlay`
  (`self.MoveAround`)
  (bind _outactors (`GameplayStatics.GetAllActorsWithTag` "PlayerChar"))
  (set `self.players` _outactors)
  (set `self.RandomIdleIndex` (`KismetMathLibrary.RandomIntegerInRange` 0 5)))

(event `self.dialogue_box.OnComponentBeginOverlap`
  (params (OverlappedComponent :type "PrimitiveComponent Object Reference") (OtherActor :type "Actor Object Reference") (OtherComp :type "PrimitiveComponent Object Reference") (OtherBodyIndex :type Integer) (bFromSweep :type Boolean) (SweepResult :type "HitResult Structure (by ref)"))
  (if (`self.ActorHasTag` OtherActor "pedestrian")
    (set `self.canTalk?` true)
    (else
      (set `self.canTalk?` false))))

(event `Talk`
  (bind _returnvalue (`SkeletalMeshComponent.GetAnimInstance` (`self.Mesh`)))
  (if (`self.canTalk?`)
    (switch `int` (`KismetMathLibrary.RandomIntegerInRange` 0 5)
      (:`0`
        (set `self.isTalking?` true)
        (`MovementComponent.StopMovementImmediately` (`self.CharacterMovement`))
        (bind _returnvalue_2 (`KismetMathLibrary.FindLookAtRotation` (`self.K2_GetActorLocation`) (`self.K2_GetActorLocation` (stale `self.dialogue_box.OnComponentBeginOverlap` OtherActor))))
        (`self.K2_SetActorRotation` _returnvalue_2 true)
        (`self.K2_SetActorRotation` (stale `self.dialogue_box.OnComponentBeginOverlap` OtherActor) _returnvalue_2 false)
        (switch `int` (`KismetMathLibrary.RandomIntegerInRange` 0 2)
          (:`0`
            (set `self.AnimationToPlay` null))
          (:`1`
            (set `self.AnimationToPlay` null))
          (:`2`
            (set `self.AnimationToPlay` null)))
        (`AnimInstance.Montage_Play` _returnvalue (`self.AnimationToPlay`) 1.0 "MontageLength" 0.0 true)
        (`KismetSystemLibrary.Delay` 10.0)
        (`AnimInstance.Montage_Stop` _returnvalue 0.0 (`self.AnimationToPlay`))
        (`self.MoveAround`)
        (set `self.isTalking?` false))
      (:`2`
        (set `self.isTalking?` false :!label _label))
      (:`3`
        (goto _label))
      (:`4`
        (goto _label))
      (:`5`
        (goto _label)))
    (else
      (goto _label))))

(event `self.CapsuleComponent.OnComponentBeginOverlap`
  (params (OverlappedComponent :type "PrimitiveComponent Object Reference") (OtherActor :type "Actor Object Reference") (OtherComp :type "PrimitiveComponent Object Reference") (OtherBodyIndex :type Integer) (bFromSweep :type Boolean) (SweepResult :type "HitResult Structure (by ref)"))
  (if (and (`ActorComponent.ComponentHasTag` OtherComp "talkbox") (`self.canTalk?`))
    _))

(event `self.ReceiveTick`
  (params (DeltaSeconds :type "Float (single-precision)")))

(event `MoveAround`
  (bind _returnvalue (`self.GetActorForwardVector`))
  (bind _returnvalue_2 (`self.GetActorRightVector`))
  (bind _returnvalue_3 (`KismetMathLibrary.RandomBool`))
  (bind _returnvalue_4 (`SkeletalMeshComponent.GetAnimInstance` (`self.Mesh`)))
  (bind _youcanmove (`self.PlayerDistance`))
  (if _youcanmove
    (`KismetSystemLibrary.Delay` (`KismetMathLibrary.RandomFloatInRange` 0.0 5.0))
    (`|AIMoveTo` self (+ (`SceneComponent.K2_GetComponentLocation` (`self.CapsuleComponent`)) (* (`KismetMathLibrary.SelectVector` (`KismetMathLibrary.SelectVector` _returnvalue (* _returnvalue -1.0) _returnvalue_3) (`KismetMathLibrary.SelectVector` _returnvalue_2 (* _returnvalue_2 -1.0) _returnvalue_3) (`KismetMathLibrary.RandomBool`)) 1000.0)) null 50.0
      (:`OnSuccess`
        (`KismetSystemLibrary.Delay` 0.1)
        (`self.MoveAround`))
      (:`OnFail`
        (switch `int` (`KismetMathLibrary.RandomIntegerInRange` 0 5)
          (:`0`
            (set `self.AnimationToPlay` null))
          (:`1`
            (set `self.AnimationToPlay` null))
          (:`2`
            (set `self.AnimationToPlay` null))
          (:`3`
            (set `self.AnimationToPlay` null))
          (:`4`
            (set `self.AnimationToPlay` null))
          (:`5`
            (set `self.AnimationToPlay` null)))
        (`AnimInstance.Montage_Play` _returnvalue_4 (`self.AnimationToPlay`) 1.0 "MontageLength" 0.0 true)
        (`self.Talk`)
        (`KismetSystemLibrary.Delay` (`KismetMathLibrary.RandomFloatInRange` 2.0 20.0))
        (`AnimInstance.Montage_Stop` _returnvalue_4 0.0 (`self.AnimationToPlay`))
        (`self.MoveAround`)))
    (else
      (`KismetSystemLibrary.Delay` 0.5)
      (`self.MoveAround`))))

(event `self.playeravoidance.OnComponentBeginOverlap`
  (params (OverlappedComponent :type "PrimitiveComponent Object Reference") (OtherActor :type "Actor Object Reference") (OtherComp :type "PrimitiveComponent Object Reference") (OtherBodyIndex :type Integer) (bFromSweep :type Boolean) (SweepResult :type "HitResult Structure (by ref)"))
  (bind _returnvalue (`self.GetActorRightVector`))
  (bind _returnvalue_2 (`self.K2_GetActorLocation`))
  (bind _returnvalue_3 (`self.K2_GetActorLocation` OtherActor))
  (bind _returnvalue_4 (* (- _returnvalue_3 _returnvalue_2) -20.0))
  (`/Engine/EditorBlueprintResources/StandardMacros.IsValid` OtherActor
    (:`Is Valid`
      (if (`self.ActorHasTag` OtherActor "PlayerChar")
        (`/Engine/EditorBlueprintResources/StandardMacros.DoOnce` false :!label _label_2
          (:`Completed`
            (`self.K2_SetActorRotation` (`KismetMathLibrary.FindLookAtRotation` _returnvalue_2 _returnvalue_3) true)
            (`self.LaunchCharacter` (+ (select `bool` (<= (`KismetMathLibrary.VSize` (`self.GetVelocity`)) 10.0) :`false` _returnvalue_4 :`true` (* _returnvalue_4 -2.0)) (* (`self.GetActorUpVector`) 50.0) (select `bool` (`KismetMathLibrary.RandomBool`) :`false` (* _returnvalue 2050.0) :`true` (* _returnvalue -2500.0))) true true)
            (bind _returnvalue_5 (`AnimInstance.Montage_Play` (`SkeletalMeshComponent.GetAnimInstance` (`self.Mesh`)) null 1.0 "MontageLength" 0.0 true))))))))

(event `self.playeravoidance.OnComponentEndOverlap`
  (params (OverlappedComponent :type "PrimitiveComponent Object Reference") (OtherActor :type "Actor Object Reference") (OtherComp :type "PrimitiveComponent Object Reference") (OtherBodyIndex :type Integer))
  (if (`self.ActorHasTag` OtherActor "PlayerChar")
    (goto _label_2 :!via `Reset`)))

(fn `PlayerDistance`
  (returns (YouCanMove :type Boolean))
  (return (`self.WasRecentlyRendered` self 0.2)))

(fn `UserConstructionScript`)