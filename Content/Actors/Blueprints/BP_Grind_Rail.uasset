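; BP_Grind_Rail is a spline-based rail actor that builds its visible, collidable geometry from the GrindRail spline.
; The construction script adds a spline mesh per segment, using configurable mesh, material and forward axis, fitted to neighboring points' local positions and tangents.
; Each piece attaches to the spline, takes a configurable collision mode and blocks all channels.
; A relative-scale step is left disconnected, and no grinding logic lives here.
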(fn `UserConstructionScript`
  (bind _splinemeshcomp (`self.SplineMeshComp`))
  (bind _grindrail (`self.GrindRail`))
  (for _index (range (+ (- (`SplineComponent.GetNumberOfSplinePoints` (`self.GrindRail`)) 2) 1))
    (bind _returnvalue (`AddComponent|NODE_AddSplineMeshComponent-0`))
    (set `self.SplineMeshComp` _returnvalue)
    (`StaticMeshComponent.SetStaticMesh` _returnvalue (`self.CustomMesh`))
    (`PrimitiveComponent.SetMaterial` (`self.SplineMeshComp`) 0 (`self.CustomMaterial`))
    (`SplineMeshComponent.SetForwardAxis` _splinemeshcomp (`self.CustomAxis`) true)
    (`SceneComponent.K2_AttachToComponent` _splinemeshcomp _grindrail "None" "KeepRelative" "KeepRelative" "KeepRelative" false)
    (bind _returnvalue_2 (+ _index 1))
    (`SplineMeshComponent.SetStartAndEnd` _splinemeshcomp (`SplineComponent.GetLocationAtSplinePoint` _grindrail _index "Local") (`SplineComponent.GetTangentAtSplinePoint` _grindrail _index "Local") (`SplineComponent.GetLocationAtSplinePoint` _grindrail _returnvalue_2 "Local") (`SplineComponent.GetTangentAtSplinePoint` _grindrail _returnvalue_2 "Local") true)
    (`PrimitiveComponent.SetCollisionEnabled` _splinemeshcomp (`self.Collision Response`))
    (`PrimitiveComponent.SetCollisionResponseToAllChannels` _splinemeshcomp "ECR_Block")))