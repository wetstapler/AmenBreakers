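; Pedestrian zone actor that populates its box with pooled AI pedestrians when the player's view target comes near.
; A fast looping timer checks view distance, using a DoOnce to fire once on entering range and re-arm beyond it.
; On firing, it teleports the first pedestrians from BP_AI_Pedestrian_Spawner's pool, bounded by SpawnNum, to random points in the box, reusing actors rather than spawning them.
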(event `self.ReceiveBeginPlay`
  (`KismetSystemLibrary.K2_SetTimerDelegate` (delegate `Display Pedestrians`) 0.01 true))

(event `Display Pedestrians`
  (bind (_returnvalue_location _returnvalue_rotation _returnvalue_scale) (`KismetMathLibrary.BreakTransform` (`self.GetTransform`)))
  (bind (_origin _boxextent) (`KismetSystemLibrary.GetComponentBounds` (`self.Box`)))
  (bind (_returnvalue_location_2 _returnvalue_rotation_2) (`KismetMathLibrary.BreakTransform` (`KismetMathLibrary.MakeTransform` (`KismetMathLibrary.RandomPointInBoundingBox` _origin _boxextent) _returnvalue_rotation _returnvalue_scale)))
  (if (> (`self.GetDistanceTo` (`Controller.GetViewTarget` (`GameplayStatics.GetPlayerController` 0))) 15000.0)
    (goto _label :!via `Reset`)
    (else
      (`/Engine/EditorBlueprintResources/StandardMacros.DoOnce` false :!label _label
        (:`Completed`
          (bind _returnvalue (`GameplayStatics.GetActorOfClass` "/Game/Actors/Blueprints/BP_AI_Pedestrian_Spawner.BP_AI_Pedestrian_Spawner_C"))
          (for _index (range (+ (`self.SpawnNum`) 1))
            (`self.K2_TeleportTo` (`|GetArrayItem` (`/Game/Actors/Blueprints/BP_AI_Pedestrian_Spawner.Pedestrian_Pool` _returnvalue) _index) _returnvalue_location_2 _returnvalue_rotation_2)))))))

(fn `UserConstructionScript`)