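; Pedestrian spawner actor that fills a box volume with AI pedestrians on BeginPlay.
; It spawns BP_Pedestrian_AI actors at random points within the Box bounds, adjusting for collisions, and stores them in PedestrianPool.
; Each gets a random skeletal mesh from the male or female civilian arrays.
; IsMale comes from a separate random roll, so it can mismatch the mesh, and ScreamingEffect is cleared either way.
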(event `self.ReceiveBeginPlay`
  (`self.Spawn`))

(event `Spawn`
  (bind (_returnvalue_location _returnvalue_rotation _returnvalue_scale) (`KismetMathLibrary.BreakTransform` (`self.GetTransform`)))
  (bind _returnvalue (`KismetMathLibrary.RandomBool`))
  (bind (_origin _boxextent) (`KismetSystemLibrary.GetComponentBounds` (`self.Box`)))
  (for _ (range (+ (`self.SpawnNum`) 1))
    (bind _returnvalue_2 (`|SpawnActorFromClass` "/Game/Actors/Blueprints/BP_Pedestrian_AI.BP_Pedestrian_AI_C" (`KismetMathLibrary.MakeTransform` (`KismetMathLibrary.RandomPointInBoundingBox` _origin _boxextent) _returnvalue_rotation _returnvalue_scale) "AdjustIfPossibleButAlwaysSpawn" "OverrideRootScale" null null))
    (`KismetArrayLibrary.Array_Add` (`self.Pedestrian_Pool`) _returnvalue_2)
    (`SkinnedMeshComponent.SetSkinnedAssetAndUpdate` (`Character.Mesh` _returnvalue_2) (select `bool` _returnvalue :`false` (`|GetArrayItem` (`self.FemaleCivArray`) (`KismetMathLibrary.RandomIntegerInRange` 0 5)) :`true` (`|GetArrayItem` (`self.MaleCivArray`) (`KismetMathLibrary.RandomIntegerInRange` 0 5))) true)
    (if _returnvalue
      (set `/Game/Actors/Blueprints/BP_Pedestrian_AI.isMale?` false _returnvalue_2)
      (set `/Game/Actors/Blueprints/BP_Pedestrian_AI.ScreamingEffect` null _returnvalue_2)
      (else
        (set `/Game/Actors/Blueprints/BP_Pedestrian_AI.isMale?` true _returnvalue_2)
        (set `/Game/Actors/Blueprints/BP_Pedestrian_AI.ScreamingEffect` null _returnvalue_2)))))

(fn `UserConstructionScript`)